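; Ritual pedestal that holds a crystal and signals when the ritual is finished.
; An overlapping crystal snaps onto an empty pedestal and is force-released from the player's grab; leaving the sphere frees the slot.
; Each placement checks all pedestals in the level, calling RitualFinished once every one is filled.
; It also spawns a Niagara beam in the crystal's color, with a timeline animating its end between crystal and ritual manager.
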(event OnComponentBeginOverlap(Sphere)
  (params (OverlappedComponent :type Primitive%20Component%20Object%20Reference) (OtherActor :type Actor%20Object%20Reference) (OtherComp :type Primitive%20Component%20Object%20Reference) (OtherBodyIndex :type Integer) (bFromSweep :type Boolean) (SweepResult :type Hit%20Result%20Structure%20%28by%20ref%29))
  (Utilities|IsValid (Variables|Default|GetCrystalOnPiedestral)
    (:Is%20Not%20Valid
      (bind _asbp_item_crystals (Utilities|Casting|CastToBP_Item_Crystals OtherActor))
      (bind _output_get (Variables|Default|SetCrystalOnPiedestral _asbp_item_crystals))
      (Transformation|AttachComponentToComponent _output_get (Variables|Default|GetCrystalPos) "None" "SnapToTarget" "SnapToTarget" "KeepWorld" true)
      (Default|ForceUngrab (Variables|Default|GetPlayerRef))
      (Variables|Default|SetAlreadyHasACrystalOn true)
      (CallFunction|CheckifAllPedestalsFilled)
      (CallFunction|TraceLinetoFlower))))

(event OnComponentEndOverlap(Sphere)
  (params (OverlappedComponent :type Primitive%20Component%20Object%20Reference) (OtherActor :type Actor%20Object%20Reference) (OtherComp :type Primitive%20Component%20Object%20Reference) (OtherBodyIndex :type Integer))
  (if (== OtherActor (Variables|Default|GetCrystalOnPiedestral))
    (Variables|Default|SetAlreadyHasACrystalOn false)
    (Variables|Default|SetCrystalOnPiedestral 0)))

(event Custom|TraceLineToFlower
  (bind _returnvalue (Niagara|SpawnSystematLocation "/Game/00-Blueprints/Lasers/NS_LightBeam.NS_LightBeam" (Transformation|GetActorLocation (Variables|Default|GetCrystalOnPiedestral))))
  (bind _output_get (Variables|Default|SetBeamEffect _returnvalue))
  (Niagara|SetNiagaraVariable(LinearColor) _output_get "Beam Color" (Variables|/Game/00-Blueprints/Items/BP_Item_Crystals.BP_Item_Crystals_C|GetLightColor (Variables|Default|GetCrystalOnPiedestral)))
  (bind _returnvalue_2 (Actor|GetActorOfClass "/Game/00-Blueprints/Items/BP_RitualManager.BP_RitualManager_C"))
  (bind _percentage (Timeline|LaserMovement PlayFromStart)
    (:Update
      (Niagara|SetNiagaraVariable(Vector3) (Variables|Default|GetBeamEffect) "Beam End" (Math|Vector|Lerp(Vector) (Transformation|GetActorLocation _returnvalue_2) (Transformation|GetActorLocation (Variables|Default|GetCrystalOnPiedestral)) _percentage)))))

(event Custom|CheckIfAllPedestalsFilled
  (bind _bool (CallFunction|AllPedestalsFilled?))
  (if _bool
    (Default|CallRitualFinished)))

(event EventBeginPlay
  (bind _asbp_fpsplayer (Utilities|Casting|CastToBP_FPSPlayer (Game|GetPlayerCharacter 0)))
  (Variables|Default|SetPlayerRef _asbp_fpsplayer))

(fn ConstructionScript
  (|CallParentFunction))

(fn AllPedestalsFilled?
  (bind _outactors (Actor|GetAllActorsOfClass "BP_Item_RitualPedestre_C"))
  (for _array_element _outactors
    (if (not (Variables|BP_Item_RitualPedestre_C|GetAlreadyHasACrystalOn _array_element))
      (return false)))
  (return true))