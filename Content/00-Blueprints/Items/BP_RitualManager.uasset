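; Manager actor that resolves the crystal ritual and picks the game's ending.
; When a pedestal signals the ritual's end, it sums crystal balances and shows a bad, neutral or good ending widget after a delay.
; Meanwhile, it spawns a ring of rotating anchors, matching each pedestal to its closest anchor direction by dot product.
; Crystals follow their anchors as a timeline drives follow and rotation speed.
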(event Custom|HandleRitualEnd
  (Development|PrintString "Ritual End")
  (Variables|Default|SetTotalBalance 0)
  (for _array_element (Variables|Default|GetRitualPedestrals)
    (Variables|Default|SetTotalBalance (+ (Variables|/Game/00-Blueprints/Items/BP_Item_Crystals.BP_Item_Crystals_C|GetBalance (Variables|/Game/00-Blueprints/Items/BP_Item_RitualPedestre.BP_Item_RitualPedestre_C|GetCrystalOnPiedestral _array_element)) (Variables|Default|GetTotalBalance))))
  (if (< (Variables|Default|GetTotalBalance) 0)
    (CallFunction|HandleNegativeBalance)
    (elif (> (Variables|Default|GetTotalBalance) 0)
      (CallFunction|HandlePositiveBalance)
      (else
        (CallFunction|HandleNeutralBalance))))
  (CallFunction|MakeCrystalsCircle))

(event Custom|HandleNeutralBalance
  (Utilities|FlowControl|Delay 1e+01)
  (Development|PrintString "Neutral Balance")
  (bind _returnvalue (UserInterface|CreateWidget "/Game/00-Blueprints/Widgets/WBP_NeutralEnding.WBP_NeutralEnding_C"))
  (UserInterface|Viewport|AddtoViewport _returnvalue 0))

(event Custom|HandleNegativeBalance
  (Utilities|FlowControl|Delay 1e+01)
  (Development|PrintString "Negative Balance")
  (bind _returnvalue (UserInterface|CreateWidget "/Game/00-Blueprints/Widgets/WBP_BadEnding.WBP_BadEnding_C"))
  (UserInterface|Viewport|AddtoViewport _returnvalue 0))

(event Custom|MakeCrystalsCircle
  (CallFunction|SetupCrystalAnchors 75.0)
  (CallFunction|ReorderAnchorsBasedonAngle)
  (for (_array_element _array_index) (Variables|Default|GetRitualPedestrals)
    (Default|MakeCrystalFollow _array_element (Utilities|Array|Get(acopy) (Variables|Default|GetCrystalAnchors) _array_index)))
  (bind (_direction _followspeed _rotationspeed) (Timeline|CrystalsCircling PlayFromStart)
    (:Update
      (Utilities|FlowControl|Sequence
        (:then_0
          (for _array_element_2 (Variables|Default|GetRitualPedestrals)
            (Variables|/Game/00-Blueprints/Items/BP_Item_Crystals.BP_Item_Crystals_C|SetFollowSpeed (Variables|/Game/00-Blueprints/Items/BP_Item_RitualPedestre.BP_Item_RitualPedestre_C|GetCrystalOnPiedestral _array_element_2) _followspeed)))
        (:then_1
          (for _array_element_3 (Variables|Default|GetCrystalAnchors)
            (Variables|/Script/Engine.RotatingMovementComponent|SetRotationRate (Variables|/Game/00-Blueprints/BP_CrystalAnchor.BP_CrystalAnchor_C|GetRotatingMovement _array_element_3) (Math|Rotator|MakeRotator 0.0 0.0 _rotationspeed))))))
    (:Finished
      (Development|PrintString "Ritual Finished"))))

(event Custom|HandlePositiveBalance
  (Utilities|FlowControl|Delay 1e+01)
  (Development|PrintString "Positive Balance")
  (bind _returnvalue (UserInterface|CreateWidget "/Game/00-Blueprints/Widgets/WBP_GoodEnding.WBP_GoodEnding_C"))
  (UserInterface|Viewport|AddtoViewport _returnvalue 0))

(event EventBeginPlay
  (bind _outactors (Actor|GetAllActorsOfClass "/Game/00-Blueprints/Items/BP_Item_RitualPedestre.BP_Item_RitualPedestre_C"))
  (bind _output_get (Variables|Default|SetRitualPedestrals _outactors))
  (for _array_element _output_get
    (EventDispatchers|BindEventtoRitualFinished _array_element (delegate Custom|HandleRitualEnd))))

(fn ConstructionScript)

(fn SetupCrystalAnchors
  (params (CircleRadius :type Float%20%28double-precision%29))
  (bind _returnvalue (Transformation|GetActorTransform))
  (LocalVariables|SetAngleStep (Math|Conversions|ToFloat(Integer) (/ 360 (Utilities|Array|Length (Variables|Default|GetRitualPedestrals)))))
  (for (_ _array_index) (Variables|Default|GetRitualPedestrals)
    (Utilities|FlowControl|Sequence
      (:then_0
        ;[0.15 0.15 0.15 0.5] Get Direction Angle Sinus and Cosinus
        (LocalVariables|SetTempCos (Math|Trig|Cos(Radians) (Math|Trig|DegreesToRadians (+ (* (LocalVariables|GetAngleStep) (+ (Math|Conversions|ToFloat(Integer) _array_index) 1.0)) 45.0))))
        (LocalVariables|SetTempSin (Math|Trig|Sin(Radians) (Math|Trig|DegreesToRadians (+ (* (LocalVariables|GetAngleStep) (+ (Math|Conversions|ToFloat(Integer) _array_index) 1.0)) 45.0)))))
      (:then_1
        (bind _returnvalue_2 (Game|SpawnActorfromClass "/Game/00-Blueprints/BP_CrystalAnchor.BP_CrystalAnchor_C" (Math|Transform|MakeTransform (.location _returnvalue) "0, 0, 0" (.scale _returnvalue)) "Undefined" "MultiplyWithRoot" 0 0))
        (Utilities|Array|AddUnique (Variables|Default|GetCrystalAnchors) _returnvalue_2)
        (Transformation|SetActorLocation _returnvalue_2 (+ (Math|Vector|MakeVector (* CircleRadius (LocalVariables|GetTempCos)) (* (LocalVariables|GetTempSin) CircleRadius) 0.0) (Transformation|GetActorLocation)) false true)
        (Variables|/Script/Engine.RotatingMovementComponent|SetPivotTranslation (Variables|/Game/00-Blueprints/BP_CrystalAnchor.BP_CrystalAnchor_C|GetRotatingMovement _returnvalue_2) (- (Transformation|GetActorLocation) (Transformation|GetActorLocation _returnvalue_2)))))))

(fn ReorderAnchorsBasedonAngle
  (bind _self self)
  (bind _returnvalue (Transformation|GetActorLocation _self))
  (for (_array_element _array_index) (Variables|Default|GetRitualPedestrals)
    (LocalVariables|SetTempBestAnchorDot 0.0)
    (for _array_element_2 (Variables|Default|GetCrystalAnchors)
      (if (> (Math|Vector|DotProduct (Math|Vector|Normalize (- _returnvalue (Transformation|GetActorLocation _array_element_2))) (Math|Vector|Normalize (- _returnvalue (Transformation|GetActorLocation _array_element)))) (LocalVariables|GetTempBestAnchorDot))
        (LocalVariables|SetTempBestAnchor _array_element_2)
        (LocalVariables|SetTempBestAnchorDot (Math|Vector|DotProduct (Math|Vector|Normalize (- _returnvalue (Transformation|GetActorLocation _array_element_2))) (Math|Vector|Normalize (- _returnvalue (Transformation|GetActorLocation _array_element)))))))
    (Utilities|Array|SetArrayElem (LocalVariables|GetNewCrystalAnchors) _array_index (LocalVariables|GetTempBestAnchor) true))
  (Variables|Default|SetCrystalAnchors (LocalVariables|GetNewCrystalAnchors)))