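; Emotion crystal item whose type sets its mesh, material, particles, light color, looping sound and balance value on BeginPlay.
; Look-at events toggle an outline decal, and PlayBalanceSound plays a positive, neutral or negative cue from that balance.
; Tick eases a held crystal toward the player's socket or moves it at constant speed toward FollowedActor.
; While following an actor, manually computed velocity drives whoosh volume and a Doppler-style pitch relative to the camera.
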(event Custom|PlayBalanceSound
  (if (== (Variables|Default|GetBalance) 1)
    (Audio|SpawnSoundAttached "/Game/02-Musics_SFX/Crystals/positive_crystal_reworked.positive_crystal_reworked" (Variables|Default|GetSM_Shape) "None" "0, 0, 0" "0, 0, 0" "KeepRelativeOffset" true 1.0 1.0 0.0 "/Game/02-Musics_SFX/SA_Crystals.SA_Crystals" 0)
    (elif (== (Variables|Default|GetBalance) 0)
      (Audio|SpawnSoundAttached "/Game/02-Musics_SFX/Crystals/neutral_crystal_reworked.neutral_crystal_reworked" (Variables|Default|GetSM_Shape) "None" "0, 0, 0" "0, 0, 0" "KeepRelativeOffset" true 1.0 1.0 0.0 "/Game/02-Musics_SFX/SA_Crystals.SA_Crystals" 0)
      (elif (== (Variables|Default|GetBalance) -1)
        (Audio|SpawnSoundAttached "/Game/02-Musics_SFX/Crystals/negative_crystal_reworked.negative_crystal_reworked" (Variables|Default|GetSM_Shape) "None" "0, 0, 0" "0, 0, 0" "KeepRelativeOffset" true 1.0 1.0 0.0 "/Game/02-Musics_SFX/SA_Crystals.SA_Crystals" 0)))))

(event Custom|DisableOutline
  ;[1 1 1] Master Item Thingy
  (Development|SetHiddeninGame (Variables|Default|GetDecal_Outline) true false))

(event Custom|EnableOutline
  ;[1 1 1] Master Item Thingy
  (Development|SetHiddeninGame (Variables|Default|GetDecal_Outline) false false))

(event EventBeginPlay
  (bind _sm_shape (Variables|Default|GetSM_Shape))
  (CallFunction|DisableOutline)
  (Variables|Default|SetPreviousLocation (Transformation|GetActorLocation))
  (bind _returnvalue (Actor|GetActorOfClass "/Game/00-Blueprints/Player/BP_FPSPlayer.BP_FPSPlayer_C"))
  (Variables|Default|SetPlayer _returnvalue)
  (switch Utilities|FlowControl|Switch|SwitchonE_CrystalsType (Variables|Default|GetCrystalType)
    (:NewEnumerator0
      (Variables|Default|SetCrystalSFX "/Game/02-Musics_SFX/Crystals/SC_Anger.SC_Anger")
      (Variables|Default|SetCrystalMesh "/Game/Crystals/Mesh/SM_Crystal_3.SM_Crystal_3")
      (Variables|Default|SetCrystalMaterial "/Game/Crystals/Material/M_Crystal_Inst3.M_Crystal_Inst3")
      (Variables|Default|SetCrystalVFX "/Game/Crystals/Particles/P_Crystal_3.P_Crystal_3")
      (Variables|Default|SetLightColor "(R=1.000000,G=0.145098,B=0.145098,A=1.000000)")
      (Variables|Default|SetBalance -1))
    (:NewEnumerator1
      (Variables|Default|SetCrystalSFX "/Game/02-Musics_SFX/Crystals/SC_Sadness.SC_Sadness")
      (Variables|Default|SetCrystalMesh "/Game/Crystals/Mesh/SM_Crystal_3.SM_Crystal_3")
      (Variables|Default|SetCrystalMaterial "/Game/Crystals/Material/M_Crystal_Inst4.M_Crystal_Inst4")
      (Variables|Default|SetCrystalVFX "/Game/Crystals/Particles/P_Crystal_5.P_Crystal_5")
      (Variables|Default|SetLightColor "(R=0.105882,G=0.454902,B=1.000000,A=1.000000)")
      (Variables|Default|SetBalance 0))
    (:NewEnumerator2
      (Variables|Default|SetCrystalSFX "/Game/02-Musics_SFX/Crystals/SC_Hope.SC_Hope")
      (Variables|Default|SetCrystalMesh "/Game/Crystals/Mesh/SM_Crystal_3.SM_Crystal_3")
      (Variables|Default|SetCrystalMaterial "/Game/Crystals/Material/M_Crystal_Inst6.M_Crystal_Inst6")
      (Variables|Default|SetCrystalVFX "/Game/Crystals/Particles/P_Crystal_7.P_Crystal_7")
      (Variables|Default|SetLightColor "(R=0.176471,G=1.000000,B=0.223529,A=1.000000)")
      (Variables|Default|SetBalance 1))
    (:NewEnumerator3
      (Variables|Default|SetCrystalSFX "/Game/02-Musics_SFX/Crystals/SC_Joy.SC_Joy")
      (Variables|Default|SetCrystalMesh "/Game/Crystals/Mesh/SM_Crystal_3.SM_Crystal_3")
      (Variables|Default|SetCrystalMaterial "/Game/Crystals/Material/M_Crystal_Inst9_2.M_Crystal_Inst9_2")
      (Variables|Default|SetCrystalVFX "/Game/Crystals/Particles/P_Crystal_9.P_Crystal_9")
      (Variables|Default|SetLightColor "(R=1.000000,G=0.905882,B=0.235294,A=1.000000)")
      (Variables|Default|SetBalance 1))
    (:NewEnumerator4
      (Variables|Default|SetCrystalSFX "/Game/02-Musics_SFX/Crystals/SC_Fear.SC_Fear")
      (Variables|Default|SetCrystalMesh "/Game/Crystals/Mesh/SM_Crystal_3.SM_Crystal_3")
      (Variables|Default|SetCrystalMaterial "/Game/Crystals/Material/M_Crystal_Inst1_2.M_Crystal_Inst1_2")
      (Variables|Default|SetCrystalVFX "/Game/Crystals/Particles/P_Crystal_1.P_Crystal_1")
      (Variables|Default|SetLightColor "(R=1.000000,G=0.266667,B=0.980392,A=1.000000)")
      (Variables|Default|SetBalance -1))
    (:NewEnumerator5
      (Variables|Default|SetCrystalSFX "/Game/02-Musics_SFX/Crystals/SC_Remission.SC_Remission")
      (Variables|Default|SetCrystalMesh "/Game/Crystals/Mesh/SM_Crystal_3.SM_Crystal_3")
      (Variables|Default|SetCrystalMaterial "/Game/Crystals/Material/M_Crystal_Inst10.M_Crystal_Inst10")
      (Variables|Default|SetCrystalVFX "/Game/Crystals/Particles/P_Crystal_10.P_Crystal_10")
      (Variables|Default|SetLightColor "(R=1.000000,G=0.356863,B=0.121569,A=1.000000)")
      (Variables|Default|SetBalance 0)))
  (Audio|SpawnSoundAttached (Variables|Default|GetCrystalSFX) (Variables|Default|GetSM_Shape) "None" "0, 0, 0" "0, 0, 0" "KeepRelativeOffset" true 1.0 1.0 0.0 "/Game/02-Musics_SFX/SA_Crystals.SA_Crystals" 0)
  (bind _returnvalue_2 (Audio|SpawnSoundAttached "/Game/02-Musics_SFX/Crystals/shut_up_ghost-smooth-cold-wind-looped-135538.shut_up_ghost-smooth-cold-wind-looped-135538" (Variables|Default|GetSM_Shape) "None" "0, 0, 0" "0, 0, 0" "KeepRelativeOffset" true 0.0 1.0 0.0 "/Game/02-Musics_SFX/SA_CrystalsWhoosh.SA_CrystalsWhoosh" 0 false))
  (Variables|Default|SetWhooshSound _returnvalue_2)
  (Components|StaticMesh|SetStaticMesh _sm_shape (Variables|Default|GetCrystalMesh))
  (Rendering|Material|SetMaterial _sm_shape 0 (Variables|Default|GetCrystalMaterial))
  (Effects|Components|ParticleSystem|SetTemplate (Variables|Default|GetP_Crystal_1) (Variables|Default|GetCrystalVFX))
  (Rendering|Components|Light|SetLightColor (Variables|Default|GetPointLight) (Variables|Default|GetLightColor) true))

(event EventTick
  (params (DeltaSeconds :type Float%20%28single-precision%29))
  (Utilities|FlowControl|Sequence
    (:then_0
      (if (Variables|Default|GetisHeld?)
        (bind _sweephitresult (Transformation|SetActorLocation (Math|Interpolation|VInterpTo (Transformation|GetActorLocation self) (Transformation|GetWorldLocation (Variables|/Game/00-Blueprints/Player/BP_FPSPlayer.BP_FPSPlayer_C|GetCrystalSocket (Variables|Default|GetPlayer))) DeltaSeconds (Variables|Default|GetFollowSpeed)) true false))
        (Development|PrintString (Utilities|String|ToString(Boolean) (.bBlockingHit (Collision|BreakHitResult _sweephitresult))))))
    (:then_1
      (Utilities|IsValid (Variables|Default|GetFollowedActor)
        (:Is%20Valid
          (Utilities|FlowControl|Sequence
            (:then_0
              ;[1 1 1] Update Pitch
              (Audio|Components|Audio|SetPitchMultiplier (Variables|Default|GetWhooshSound) (Math|Float|Clamp(Float) (/ (Variables|Default|GetSpeedOfSound) (- (Variables|Default|GetSpeedOfSound) (Math|Vector|DotProduct (/ (- (Transformation|GetActorLocation) (Variables|Default|GetPreviousLocation)) DeltaSeconds) (Math|Vector|Normalize (- (Transformation|GetWorldLocation (Variables|/Game/00-Blueprints/Player/BP_FPSPlayer.BP_FPSPlayer_C|GetFirstPersonCamera (Variables|Default|GetPlayer))) (Transformation|GetActorLocation)))))) 0.5 1.5)))
            (:then_1
              ;[1 1 1] Calculate manual velocity
              (Variables|Default|SetVelocity (/ (Math|Vector|VectorLength (- (Variables|Default|GetPreviousLocation) (Transformation|GetActorLocation))) DeltaSeconds))
              (Variables|Default|SetPreviousLocation (Transformation|GetActorLocation)))
            (:then_2
              ;[1 1 1] Make the crystal follow the followed actor
              (Utilities|IsValid (Variables|Default|GetFollowedActor)
                (:Is%20Valid
                  (Transformation|SetActorLocation (Math|Interpolation|VInterptoConstant (Transformation|GetActorLocation self) (Transformation|GetActorLocation (Variables|Default|GetFollowedActor)) DeltaSeconds (Variables|Default|GetFollowSpeed)) false false))))
            (:then_3
              ;[1 1 1] Varying Volumen Based on Manual Velocity
              (Utilities|IsValid (Variables|Default|GetWhooshSound)
                (:Is%20Valid
                  (Audio|Components|Audio|SetVolumeMultiplier (Variables|Default|GetWhooshSound) (Math|Float|MapRangeClamped (Variables|Default|GetVelocity) 0.0 8e+02 0.0 1.2) :!class /Script/Engine.AudioComponent))))))))))

(event EventStartLookatInteractables
  ;[1 1 1] Master Item Thingy
  (Utilities|FlowControl|DoOnce false
    (:Completed
      (CallFunction|EnableOutline))))

(event EventStopLookatInteractables
  ;[1 1 1] Master Item Thingy
  (Utilities|FlowControl|Sequence
    (:then_0
      (Utilities|FlowControl|DoOnce false) ; enters at Reset
    )
    (:then_1
      (CallFunction|DisableOutline))))

(fn ConstructionScript)